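; Player controller that lets a DualShock 4, read as a generic USB controller, fly the controlled pawn with six degrees of freedom.
; BeginPlay adds the input config, logs raw devices and flags "05C4" pads as first generation, though IsFirstGeneration is set false.
; Deadzoned axes drive pitch, yaw and movement along control-rotation vectors, with centred axes remapped to ±1.
; Buttons 5 and 6 roll through looping timers while held.
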(event Custom|RollRight
  (Class|PlayerController|AddRollInput 1.0))

(event Custom|RollLeft
  (Class|PlayerController|AddRollInput (Game|GetPlayerController 0) -1.0))

(event EventBeginPlay
  (bind _returnvalue (Game|GetPlayerController 0))
  (Class|EnhancedInputSubsystemInterface|AddPlayerMappableConfig (PlayerController|LocalPlayerSubsystems|GetEnhancedInputLocalPlayerSubsystem _returnvalue) "/Game/DualShock4/IMP_DualShock4.IMP_DualShock4" (Utilities|Struct|MakeModifyContextOptions false false))
  (CallFunction|DetectFirstGeneration)
  (CallFunction|LogRegisteredDevices)
  (Input|SetInputModeGameOnly _returnvalue true))

(event Input|AxisEvents|InputAxisGenericUSBControllerAxis3
  (params (AxisValue :type Float%20%28single-precision%29))
  (bind _returnvalue (- AxisValue 0.5))
  (bind _returnvalue_2 (* _returnvalue 2.0))
  (if (not (<= (Math|Float|Absolute(Float) _returnvalue_2) 0.05))
    (Class|PlayerController|AddPitchInput (Game|GetPlayerController 0) _returnvalue_2)))

(event Input|AxisEvents|InputAxisGenericUSBControllerAxis5
  (params (AxisValue :type Float%20%28single-precision%29))
  (bind _returnvalue (Game|GetPlayerController 0))
  (bind _returnvalue_2 (- AxisValue 0.5))
  (bind _returnvalue_3 (* _returnvalue_2 -2.0))
  (if (not (<= (Math|Float|Absolute(Float) _returnvalue_3) 0.05))
    (Pawn|Input|AddMovementInput (Pawn|GetControlledPawn _returnvalue) (Math|Vector|GetUpVector (Math|Rotator|MakeRotator 0.0 0.0 (.yaw (Pawn|GetControlRotation _returnvalue :!class /Script/Engine.Controller)))) _returnvalue_3 false)))

(event Input|AxisEvents|InputAxisGenericUSBControllerAxis6
  (params (AxisValue :type Float%20%28single-precision%29))
  (bind _returnvalue (Game|GetPlayerController 0))
  (bind _returnvalue_2 (- AxisValue 0.5))
  (bind _returnvalue_3 (Pawn|GetControlRotation _returnvalue :!class /Script/Engine.Controller))
  (bind _returnvalue_4 (* _returnvalue_2 2.0))
  (if (not (<= (Math|Float|Absolute(Float) _returnvalue_4) 0.05))
    (Pawn|Input|AddMovementInput (Pawn|GetControlledPawn _returnvalue) (Math|Vector|GetRightVector (Math|Rotator|MakeRotator (.roll _returnvalue_3) 0.0 (.yaw _returnvalue_3))) _returnvalue_4 false)))

(event Input|AxisEvents|InputAxisGenericUSBControllerAxis4
  (params (AxisValue :type Float%20%28single-precision%29))
  (bind _returnvalue (- AxisValue 0.5))
  (bind _returnvalue_2 (* _returnvalue 2.0))
  (if (not (<= (Math|Float|Absolute(Float) _returnvalue_2) 0.05))
    (Class|PlayerController|AddYawInput (Game|GetPlayerController 0) _returnvalue_2)))

(event Input|AxisEvents|InputAxisGenericUSBControllerAxis2
  (params (AxisValue :type Float%20%28single-precision%29))
  (bind _returnvalue (Game|GetPlayerController 0))
  (bind _returnvalue_2 (Pawn|GetControlRotation _returnvalue :!class /Script/Engine.Controller))
  (Development|PrintString (Utilities|String|ToString(Float) AxisValue) true true "(R=0.000000,G=0.660000,B=1.000000,A=1.000000)" 2.0 "Axis2")
  (if (not (<= (Math|Float|Absolute(Float) AxisValue) 0.05))
    (Pawn|Input|AddMovementInput (Pawn|GetControlledPawn _returnvalue) (Math|Vector|GetForwardVector (Math|Rotator|MakeRotator (.roll _returnvalue_2) (.pitch _returnvalue_2) (.yaw _returnvalue_2))) (* AxisValue -1.0) false)))

(event Input|AxisEvents|InputAxisGenericUSBControllerAxis1
  (params (AxisValue :type Float%20%28single-precision%29))
  (bind _returnvalue (Game|GetPlayerController 0))
  (bind _returnvalue_2 (Pawn|GetControlRotation _returnvalue :!class /Script/Engine.Controller))
  (if (not (<= (Math|Float|Absolute(Float) AxisValue) 0.05))
    (Pawn|Input|AddMovementInput (Pawn|GetControlledPawn _returnvalue) (Math|Vector|GetForwardVector (Math|Rotator|MakeRotator (.roll _returnvalue_2) (.pitch _returnvalue_2) (.yaw _returnvalue_2))) AxisValue false)))

(event Input|KeyboardEvents|GenericUSBControllerButton5
  (params (Key :type Key%20Structure :default "None"))
  (:Pressed
    (bind _returnvalue (Utilities|Time|SetTimerbyEvent (delegate Custom|RollLeft) (Utilities|Time|GetWorldDeltaSeconds) true)))
  (:Released
    (Utilities|Time|ClearandInvalidateTimerbyHandle _returnvalue)))

(event Input|KeyboardEvents|GenericUSBControllerButton6
  (params (Key :type Key%20Structure :default "None"))
  (:Pressed
    (bind _returnvalue (Utilities|Time|SetTimerbyEvent (delegate Custom|RollRight) (Utilities|Time|GetWorldDeltaSeconds) true)))
  (:Released
    (Utilities|Time|ClearandInvalidateTimerbyHandle _returnvalue)))

(fn ConstructionScript)

(fn LogRegisteredDevices
  (for (_array_element _array_index) (Class|RawInputFunctionLibrary|GetRegisteredDevices)
    (Development|PrintString (Utilities|String|Append "Handle : " (Utilities|String|ToString(Integer) (.handle _array_element)) "  
" "VendorID : " (Utilities|String|ToString(Integer) (.vendorid _array_element)) "  
" "ProductID : " (Utilities|String|ToString(Integer) (.productid _array_element)) "  
" "DeviceName : " (.devicename _array_element) "  
" "ArrayIndex : " (Utilities|String|ToString(Integer) _array_index)) true true "(R=0.000000,G=0.660000,B=1.000000,A=1.000000)" 1e+01)
    (if (Utilities|String|Contains (.devicename _array_element) "05C4")
      (Variables|Default|SetbIsFirstGeneration false))))

(fn DetectFirstGeneration
  (for _array_element (Class|RawInputFunctionLibrary|GetRegisteredDevices)
    (if (Utilities|String|Contains (.devicename _array_element) "05C4")
      (Variables|Default|SetbIsFirstGeneration false)
      (Development|PrintString "!!! FIRST GENERATION DUALSHOCK4 !!!"))))